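; BP_Player is the player character, providing movement, look, free look and pose/move state functions.
; Tick calls CallOnMoveChanged whenever velocity starts or stops being non-zero, while UpdateMoveState resolves input flags by priority: Aim, Walk, Run, then Jog.
; Free look unlocks controller yaw and keeps movement relative to the saved starting yaw.
; On release, a timeline lerps control rotation back along the shortest path, then restores controller yaw.
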(event EventTick
  (params (DeltaSeconds :type Float%20%28single-precision%29))
  (bind _returnvalue (Transformation|GetVelocity))
  (bind _returnvalue_2 (Math|Vector|VectorLengthSquared _returnvalue))
  (bind _returnvalue_3 (> _returnvalue_2 0.0))
  (if (!= (Variables|Move|GetbIsMoving) _returnvalue_3)
    (bind _output_get (Variables|Move|SetbIsMoving _returnvalue_3))
    (Default|CallOnMoveChanged _output_get)))

(event Custom|OnFreeLookEnded
  (bind _alpha (Timeline|TL_OnFreeLookEnded PlayFromStart)
    (:Update
      (Pawn|SetControlRotation (Pawn|GetController) (Math|Rotator|Lerp(Rotator) (Variables|FreeLook|GetFreeLookEndRotation) (Variables|FreeLook|GetFreeLookStartRotation) _alpha true)))
    (:Finished
      (Variables|Default|SetbUseControllerRotationYaw true))))

(fn ConstructionScript)

(fn InputTurn
  (params (XAxisValue :type Float%20%28double-precision%29))
  (Pawn|Input|AddControllerYawInput XAxisValue))

(fn InputLookUp
  (params (YAxisValue :type Float%20%28double-precision%29))
  (Pawn|Input|AddControllerPitchInput YAxisValue))

(fn Move
  (params (bIsForward :type Boolean) (AxisValue :type Float%20%28double-precision%29))
  (bind _yawonlyrotator (Movement|GetMoveRotation))
  (if bIsForward
    (Pawn|Input|AddMovementInput (Math|Vector|GetForwardVector _yawonlyrotator) AxisValue false)
    (else
      (Pawn|Input|AddMovementInput (Math|Vector|GetRightVector _yawonlyrotator) AxisValue false))))

(fn FreeLook
  (params (bIsPressed :type Boolean))
  (bind _returnvalue (Pawn|GetControlRotation :!class /Script/Engine.Pawn))
  (if bIsPressed
    (Variables|FreeLook|SetFreeLookStartRotation _returnvalue)
    (Variables|Default|SetbUseControllerRotationYaw false)
    (else
      (Variables|FreeLook|SetFreeLookEndRotation _returnvalue)
      (CallFunction|OnFreeLookEnded))))

(fn GetMoveRotation
  (return (Math|Rotator|SelectRotator (CallFunction|GetYawOnlyRotator (Pawn|GetControlRotation :!class /Script/Engine.Pawn)) (CallFunction|GetYawOnlyRotator (Variables|FreeLook|GetFreeLookStartRotation)) (Variables|Default|GetbUseControllerRotationYaw))))

(fn UpdatePoseState
  (params (NewState :type E_PoseState%20Enum :default "NewEnumerator0"))
  (Variables|Pose|SetCurrentPoseState NewState))

(fn UpdateMoveState
  ;[0.15 0.15 0.15 0.5] 우선순위 Aim -> Walk -> Run -> Jog
  (if (Variables|Move|GetbIsAimPressed)
    (Variables|Move|SetCurrentMoveState "NewEnumerator3")
    (elif (Variables|Move|GetbIsWalkPressed)
      (Variables|Move|SetCurrentMoveState "NewEnumerator0")
      (elif (Variables|Move|GetbIsRunPressed)
        (Variables|Move|SetCurrentMoveState "NewEnumerator2")
        (else
          (Variables|Move|SetCurrentMoveState "NewEnumerator1"))))))

(fn UpdateMaxWalkSpeed
  (params (NewSpeed :type Float%20%28double-precision%29))
  (Variables|/Script/Engine.CharacterMovementComponent|SetMaxWalkSpeed (Variables|Character|GetCharacterMovement) NewSpeed))
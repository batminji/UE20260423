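; BP_WorldItem_Ammo is an ammo world item that takes its data from the DT_WorldItem_Ammo data table.
; Init calls the parent, then looks up the row by ID to pass item type, name, UI prefix and mesh to InitWorldItemBaseData.
; The same row sets the pickup amount and per-unit weight, which GetWeight multiplies to return the total weight.
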(event EventBeginPlay
  (|CallParentFunction) ; This node is disabled and will not be called.\nDrag off pins to build functionality.
)

(fn ConstructionScript
  (|CallParentFunction))

(fn Init
  (params (InID :type Name :default "None") (InSerialNumber :type String))
  (|CallParentFunction InID InSerialNumber)
  (bind _returnvalue (Utilities|GetDataTableRow "/Game/_Blueprints/Data/DataTable/Item/DT_WorldItem_Ammo.DT_WorldItem_Ammo" (Variables|Default|GetID))
    (:then
      (CallFunction|InitWorldItemBaseData (.itemtype _returnvalue) (.itemname _returnvalue) (.uiprefix _returnvalue) (.staticmesh _returnvalue))
      (Variables|Default|SetAmount (.pickupammo _returnvalue))
      (Variables|Default|SetWeight (.weight _returnvalue)))))

(fn GetWeight
  (return (* (Variables|Default|GetAmount) (Variables|Default|GetWeight))))